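; Configurable fire and explosion effect Blueprint with a point light and an animated skeletal mesh.
; The construction script applies light, template and scale settings; Tick fires once when Enabled, waiting before triggering the light, explosion particle and animation.
; A timeline then updates the fire's "dir" parameter from an oscillating or fixed direction plus random jitter, reactivating it and toggling smoke and distortion emitters.
; The Explode function is empty.
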(event EventTick
  (params (DeltaSeconds :type Float%20%28single-precision%29))
  (bind _fire_particle (Variables|Default|GetFire_particle))
  (bind _random_start_angle_max (Variables|Fire_Angle|GetRandom_Start_angle_max))
  (bind _random_start_angle_min (Variables|Fire_Angle|GetRandom_Start_angle_min))
  (bind _returnvalue (Math|Random|RandomFloatinRange _random_start_angle_min _random_start_angle_max))
  (bind _returnvalue_2 (Math|Vector|MakeVector _returnvalue _returnvalue 0.0))
  (if (Variables|Default|Getenabled)
    (Variables|Default|Setenabled false)
    (Utilities|FlowControl|Delay (Variables|FireSettings|GetExplosion_start_Delay))
    (Rendering|SetVisibility (Variables|Default|GetPointLight) (Variables|FireLight|GetLight) false)
    (Components|Activation|Activate (Variables|Default|GetExplosion_particle) false)
    (Components|Animation|PlayAnimation (Variables|Default|GetSkeletalMesh) (Variables|FireSettings|GetAni_Seq) false)
    (Components|Timeline|SetPlayRate (Variables|Default|GetTimeline_0) (Variables|Fire_Oscillator|GetOscil_Speed))
    (bind _dir_vector (Timeline|Timeline_0 Play)
      (:Update
        (Effects|Components|ParticleSystem|SetVectorParameter _fire_particle "dir" (select (Variables|Fire_Oscillator|Getoscillate) (Math|Vector|Normalize (+ _dir_vector _returnvalue_2)) (Math|Vector|Normalize (+ (Variables|FireTransform|GetDirection) _returnvalue_2))))
        (Effects|Components|ParticleSystem|SetActorParameter _fire_particle "BoneSocketActor" (Components|GetOwner _fire_particle))
        (Components|Activation|Activate _fire_particle false)
        (Effects|Components|ParticleSystem|SetEmitterEnable (Variables|Default|GetFire_particle) "smoke" (Variables|FireSettings|GetSmoke_Emitter_Enable))
        (Effects|Components|ParticleSystem|SetEmitterEnable (Variables|Default|GetFire_particle) "Distortion" (Variables|FireSettings|GetDistortion_Emittter_Enable))))))

(event EventBeginPlay)

(fn ConstructionScript
  (Rendering|Components|Light|SetIntensity (Variables|Default|GetPointLight) (Variables|FireLight|GetLight_Intensity))
  (Rendering|Lighting|SetAttenuationRadius (Variables|Default|GetPointLight) (Variables|FireLight|GetLightRadius))
  (Transformation|SetWorldLocation (Variables|Default|GetFire_particle) (Transformation|GetActorLocation) false false)
  (Effects|Components|ParticleSystem|SetTemplate (Variables|Default|GetFire_particle) (Variables|FireSettings|Getparticle_Fire))
  (Transformation|SetWorldScale3D (Variables|Default|GetFire_particle) (Variables|FireTransform|GetFire_Scale))
  (Transformation|SetWorldTransform (Variables|Default|GetExplosion_particle) (Math|Transform|MakeTransform (Transformation|GetActorLocation) "0, 0, 0" (Variables|FireTransform|GetExplosion_Scale)) false false)
  (Effects|Components|ParticleSystem|SetTemplate (Variables|Default|GetExplosion_particle) (Variables|FireSettings|Getparticle_Exp)))

(fn Explode)