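; Base locked door that is removed from the level when a player holds a matching key.
; OpenDoorWithKey loops over the player's inventory and spawns each key item's class to compare its ID with KeyID.
; On a match it calls UseItem and, if successful, decrements the slot's quantity and destroys both key actor and door.
; Non-matching spawned keys are not destroyed here; event graph is empty.
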(event EventBeginPlay)

(event Collision|EventActorBeginOverlap
  (params (OtherActor :type Actor%20Object%20Reference)))

(event EventTick
  (params (DeltaSeconds :type Float%20%28single-precision%29)))

(fn ConstructionScript)

(fn OpenDoorwithKey
  (params (player :type Third%20Person%20Character%20Object%20Reference))
  (bind _inventorycomponent (Variables|/Game/ThirdPersonBP/Blueprints/ThirdPersonCharacter.ThirdPersonCharacter_C|GetInventoryComponent player))
  (bind (_array_element _array_index) (Utilities|Array|ForEachLoopwithBreak (Variables|/Game/InventorySystem/InventoryComponent.InventoryComponent_C|GetInventory _inventorycomponent))
    (:LoopBody
      (bind _asitem_key (Utilities|Casting|CastToItem_KeyClass (.class (.itemstructure _array_element))))
      (bind _returnvalue (Game|SpawnActorfromClass _asitem_key (Math|Transform|MakeTransform "0, 0, 0" "0, 0, 0" "0.000000,0.000000,0.000000") "Undefined" 0 0))
      (if (== (Variables|/Game/InventorySystem/Items/Key/Item_Key.Item_Key_C|GetID _returnvalue) (Variables|Default|GetKeyID))
        (bind _asitem (Utilities|Casting|CastToItem _returnvalue))
        (Variables|/Game/InventorySystem/Items/Item.Item_C|SetItemStructure _asitem (Utilities|Struct|MakeItemStructure (.name (Variables|/Game/InventorySystem/Items/Item.Item_C|GetItemStructure _asitem)) (.isstackable (Variables|/Game/InventorySystem/Items/Item.Item_C|GetItemStructure _asitem)) (.thumbnail (Variables|/Game/InventorySystem/Items/Item.Item_C|GetItemStructure _asitem)) (.maxstacksize (Variables|/Game/InventorySystem/Items/Item.Item_C|GetItemStructure _asitem)) true (.duability (Variables|/Game/InventorySystem/Items/Item.Item_C|GetItemStructure _asitem)) (.description (Variables|/Game/InventorySystem/Items/Item.Item_C|GetItemStructure _asitem)) (.class (Variables|/Game/InventorySystem/Items/Item.Item_C|GetItemStructure _asitem))))
        (bind _success (Default|UseItem _returnvalue))
        (if (and _success true)
          (Utilities|Array|SetArrayElem (Variables|/Game/InventorySystem/InventoryComponent.InventoryComponent_C|GetInventory _inventorycomponent) _array_index (Utilities|Struct|MakeSlotStructure "(Name_2_B0B6932542E393C4F30619B92B9467D7=NSLOCTEXT(\"[F761C3BA4017F6B3912222A4811ED4AC]\", \"7C55D0024ADEC81212E124AD0B4CCA0C\", \"None\"),IsStackable_5_677C59A24E3749EAC0FFBF84E8687879=True,Thumbnail_8_B24175CC4A721AD669FEC0AA419E5A9D=None,MaxStackSize_11_B706B4C6403C54FAE573C2998CAB3E66=4,IsConsumable_14_96E04A944F9EA6442BC61D9EAAEBACFA=True,Duability_17_723B36744B5374B52B63029AA25E2B93=0.000000,Description_20_91B5778F49F58262C69348AC5DADE219=NSLOCTEXT(\"[F761C3BA4017F6B3912222A4811ED4AC]\", \"E7B70DB5415CE449022CD9A93B156DBF\", \"None\"),Class_23_B50496704E7C639AE8CE9FAB5E3319D3=None)" (- (.quantity (Utilities|Array|Get(acopy) (Variables|/Game/InventorySystem/InventoryComponent.InventoryComponent_C|GetInventory _inventorycomponent) _array_index)) 1)))
          (Actor|DestroyActor _returnvalue)
          (Actor|DestroyActor))))))